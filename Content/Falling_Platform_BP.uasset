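; Falling platform actor that drops under physics shortly after the player character steps on its trigger.
; The overlap starts a randomized short timer, which enables physics on the mesh and disables collision, then stops physics and hides the actor after a delay.
; ResetPlatform, when flagged as a falling platform, restores the location saved at BeginPlay, collision and visibility; its moving-platform branch is empty.
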(event `self.ReceiveBeginPlay`
  (set `self.Falling Platform Location` (`self.K2_GetActorLocation`)))

(event `self.FallingPlatformTrigger.OnComponentBeginOverlap`
  (params (OverlappedComponent :type "PrimitiveComponent Object Reference") (OtherActor :type "Actor Object Reference") (OtherComp :type "PrimitiveComponent Object Reference") (OtherBodyIndex :type Integer) (bFromSweep :type Boolean) (SweepResult :type "HitResult Structure (by ref)"))
  (if (== OtherActor (`GameplayStatics.GetPlayerCharacter` 0))
    (set `self.Standing On Platform` true)
    (bind _returnvalue (`KismetSystemLibrary.K2_SetTimerDelegate` (delegate `Platform Falls`) (`KismetMathLibrary.RandomFloatInRange` 0.7 1.5)))))

(event `Platform Falls`
  (if (`self.Standing On Platform`)
    (`PrimitiveComponent.SetSimulatePhysics` (`self.FallingPlatform_SM`) true)
    (`self.SetActorEnableCollision` false))
  (`KismetSystemLibrary.K2_ClearAndInvalidateTimerHandle` (stale `self.FallingPlatformTrigger.OnComponentBeginOverlap` _returnvalue))
  (`KismetSystemLibrary.Delay` 2.0)
  (`PrimitiveComponent.SetSimulatePhysics` (`self.FallingPlatform_SM`) false)
  (`self.SetActorHiddenInGame` true))

(event `Reset Platform`
  (if (`self.isFallingPlatform`)
    (`self.ResetFallingPlatform`)
    (if (`self.isMovingPlatform`)
      _)))

(event `ResetFallingPlatform`
  (`self.K2_SetActorLocation` (`self.Falling Platform Location`))
  (`self.SetActorEnableCollision` true)
  (`self.SetActorHiddenInGame` false))

(fn `UserConstructionScript`)