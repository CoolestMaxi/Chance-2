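; Parkour platform obstacle that can be configured through flags as moving, falling and/or invisible.
; Moving platforms run on InterpToMovement, while falling ones drop via physics shortly after the player overlaps their trigger, losing collision and later hiding.
; InvisPlatformLogic toggles visibility by swapping materials, which also mark falling platforms as broken.
; ResetPlatform teleports the actor to its starting location and restores falling and moving states.
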(event `InvisPlatformLogic`
  (params (value :type Boolean))
  (set `self.canSeeInvisible` value)
  (`self.AssignMaterials`))

(event `MovingPlatformLogic`
  (`ActorComponent.Activate` (`self.InterpToMovement`) true))

(event `FallingPlatformLogic`
  (set `self.Standing On Platform` true)
  (`KismetSystemLibrary.Delay` 0.3)
  (if (`self.Standing On Platform`)
    (if (`self.isMovingPlatform`)
      (`ActorComponent.Deactivate` (`self.InterpToMovement`)))
    (`PrimitiveComponent.SetSimulatePhysics` (`self.FallingPlatform_SM`) true)
    (`self.SetActorEnableCollision` false)
    (`KismetSystemLibrary.Delay` 2.0)
    (if (`self.Standing On Platform`)
      (`PrimitiveComponent.SetSimulatePhysics` (`self.FallingPlatform_SM`) false)
      (`self.SetActorHiddenInGame` true))))

(event `self.ReceiveBeginPlay`
  (set `self.Falling Platform Location` (`self.K2_GetActorLocation`))
  (`self.AssignMaterials`)
  (if (`self.isMovingPlatform`)
    (`self.MovingPlatformLogic`)))

(event `self.FallingPlatformTrigger.OnComponentBeginOverlap`
  (params (OverlappedComponent :type "PrimitiveComponent Object Reference") (OtherActor :type "Actor Object Reference") (OtherComp :type "PrimitiveComponent Object Reference") (OtherBodyIndex :type Integer) (bFromSweep :type Boolean) (SweepResult :type "HitResult Structure (by ref)"))
  (if (== OtherActor (`GameplayStatics.GetPlayerCharacter` 0))
    (if (`self.isFallingPlatform`)
      (`self.FallingPlatformLogic`))))

(event `Reset Platform`
  (`self.K2_SetActorLocation` (`self.Falling Platform Location`) false true)
  (if (`self.isFallingPlatform`)
    (`self.ResetFallingPlatform`))
  (if (`self.isMovingPlatform`)
    (`self.ResetMovingPlatform`)))

(event `AssignMaterials`
  (`PrimitiveComponent.SetMaterial` (`self.FallingPlatform_SM`) 0 "/Game/Obstacles/parkour_peice_mat.parkour_peice_mat")
  (if (`self.isFallingPlatform`)
    (`PrimitiveComponent.SetMaterial` (`self.FallingPlatform_SM`) 0 "/Game/Obstacles/parkour_peice_broken_mat.parkour_peice_broken_mat"))
  (if (and (`self.isInvisiblePlatform`) (!= (`self.canSeeInvisible`) true))
    (`PrimitiveComponent.SetMaterial` (`self.FallingPlatform_SM`) 0 "/Game/Obstacles/parkour_piece_invisible.parkour_piece_invisible")))

(event `ResetFallingPlatform`
  (`self.SetActorEnableCollision` true)
  (`self.SetActorHiddenInGame` false)
  (`PrimitiveComponent.SetSimulatePhysics` (`self.FallingPlatform_SM`) false)
  (set `self.Standing On Platform` false))

(event `ResetMovingPlatform`
  (bind _interptomovement (`self.InterpToMovement`))
  (`ActorComponent.Deactivate` (`self.InterpToMovement`))
  (`KismetSystemLibrary.Delay` 0.2)
  (`self.K2_SetActorLocation` (`self.Falling Platform Location`) false true)
  (`ActorComponent.Activate` _interptomovement true)
  (`InterpToMovementComponent.RestartMovement` _interptomovement 1.0))

(fn `UserConstructionScript`)